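; Builds a hexagonal room floor procedurally with Geometry Script when play begins.
; GenerateMesh resets the dynamic mesh, appends a six-sided disc sized by RoomRadius, extrudes it by FloorHeight and rotates it to a fixed orientation.
; It then generates convex-hull simple collision for the component and copies the result into the SM_Floor static mesh asset.
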(event Custom|GenerateMesh
  ;[0.15 0.15 0.15 0.5] Reset mesh
  (bind _returnvalue (DynamicMeshComponent|GetDynamicMesh (Variables|DynamicMeshActor|GetDynamicMeshComponent)))
  (DynamicMesh|Reset _returnvalue)
  (Class|GeometryScriptLibraryCollisionFunctions|ResetDynamicMeshCollision (Variables|DynamicMeshActor|GetDynamicMeshComponent) false 0)
  (Variables|Default|SetWallMesh _returnvalue)
  ;[0.15 0.15 0.15 0.5] Create walls
  (bind _returnvalue_2 (GeometryScript|Primitives|AppendDisc :TargetMesh (Variables|Default|GetWallMesh) :Radius (Variables|Default|GetRoomRadius) :AngleSteps 6 :Debug 0))
  (bind _returnvalue_3 (Class|GeometryScriptLibraryMeshModelingFunctions|ApplyMeshExtrudeCompatibility5p0 _returnvalue_2 (Utilities|Struct|MakeGeometryScriptMeshExtrudeOptions 1.0 (Math|Vector|MakeVector 0.0 0.0 (Variables|Default|GetFloorHeight)) 1.0 true) 0))
  (bind _returnvalue_4 (Class|GeometryScriptLibraryMeshTransformFunctions|RotateMesh _returnvalue_3 "0.000000,-30.000000,0.000000" "0.000000,0.000000,0.000000" 0))
  (bind _returnvalue_5 (Class|GeometryScriptLibraryCollisionFunctions|GenerateCollisionfromMesh _returnvalue_4 (Utilities|Struct|MakeGeometryScriptCollisionfromMeshOptions true "ConvexHulls") 0))
  (Class|GeometryScriptLibraryCollisionFunctions|SetSimpleCollisionOfDynamicMeshComponent :SimpleCollision _returnvalue_5 :DynamicMeshComponent (Variables|DynamicMeshActor|GetDynamicMeshComponent) :Debug 0)
  (GeometryScript|StaticMesh|CopyMeshtoStaticMesh :FromDynamicMesh _returnvalue_4 :ToStaticMeshAsset "/Game/Rooms/SM_Floor.SM_Floor" :Debug 0))

(event EventBeginPlay
  (CallFunction|GenerateMesh))

(fn ConstructionScript)