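; Generated dynamic mesh actor that builds a hexagonal room floor from a radius and height.
; GenerateMesh runs on editor rebuild and BeginPlay, using Geometry Script to extrude a six-step disc upward and rotate it.
; It derives simple collision from the result for the component.
; Each run also calls static mesh asset creation to bake the mesh to SM_Floor, with complex-as-simple collision.
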(event Custom|GenerateMesh
  ;[0.15 0.15 0.15 0.5] Reset mesh
  (bind _returnvalue (DynamicMeshComponent|GetDynamicMesh (Variables|DynamicMeshActor|GetDynamicMeshComponent)))
  (DynamicMesh|Reset _returnvalue)
  (Class|GeometryScriptLibraryCollisionFunctions|ResetDynamicMeshCollision (Variables|DynamicMeshActor|GetDynamicMeshComponent) false 0)
  (Variables|Default|SetWallMesh _returnvalue)
  ;[0.15 0.15 0.15 0.5] Create walls
  (bind _returnvalue_2 (GeometryScript|Primitives|AppendDisc :TargetMesh (Variables|Default|GetWallMesh) :Radius (Variables|Default|GetRoomRadius) :AngleSteps 6 :Debug 0))
  (bind _returnvalue_3 (Class|GeometryScriptLibraryMeshModelingFunctions|ApplyMeshExtrudeCompatibility5p0 _returnvalue_2 (Utilities|Struct|MakeGeometryScriptMeshExtrudeOptions 1.0 (Math|Vector|MakeVector 0.0 0.0 (Variables|Default|GetFloorHeight)) 1.0 true) 0))
  (bind _returnvalue_4 (Class|GeometryScriptLibraryMeshTransformFunctions|RotateMesh _returnvalue_3 "0.000000,-30.000000,0.000000" "0.000000,0.000000,0.000000" 0))
  (bind _returnvalue_5 (Class|GeometryScriptLibraryCollisionFunctions|GenerateCollisionfromMesh :FromDynamicMesh _returnvalue_4 :Debug 0))
  (Class|GeometryScriptLibraryCollisionFunctions|SetSimpleCollisionOfDynamicMeshComponent :SimpleCollision _returnvalue_5 :DynamicMeshComponent (Variables|DynamicMeshActor|GetDynamicMeshComponent) :Debug 0)
  (GeometryScript|AssetManagement|CreateNewStaticMeshAssetfromMesh (Variables|Default|GetWallMesh) "/Game/Rooms/SM_Floor" (Utilities|Struct|MakeGeometryScriptCreateNewStaticMeshAssetOptions false false false "(bEnabled=False,bPreserveArea=False,bExplicitTangents=False,bLerpUVs=True,bSeparable=False,bVoxelNDF=True,bVoxelOpacity=False,PositionPrecision=-2147483648,NormalPrecision=-1,TangentPrecision=-1,BoneWeightPrecision=-1,TargetMinimumResidencyInKB=0,KeepPercentTriangles=1.000000,TrimRelativeError=0.000000,GenerateFallback=PlatformDefault,FallbackTarget=Auto,FallbackPercentTriangles=1.000000,FallbackRelativeError=1.000000,MaxEdgeLengthFactor=0.000000,NumRays=1,VoxelLevel=0,RayBackUp=0.000000,DisplacementUVChannel=0,DisplacementMaps=,NaniteAssemblyData=(Parts=,Nodes=))" 0.0 true "CTF_UseComplexAsSimple") 0))

(event Events|EventOnRebuildGeneratedMesh
  (params (TargetMesh :type Dynamic%20Mesh%20Object%20Reference))
  (CallFunction|GenerateMesh))

(event EventBeginPlay
  (CallFunction|GenerateMesh))

(fn ConstructionScript)