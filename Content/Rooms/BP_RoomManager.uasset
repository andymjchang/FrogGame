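; BP_RoomManager places rooms on a hex grid, using a selector room steered by keyboard.
; BeginPlay calls PlaceRoom twice and spawns hidden grid markers at valid hexes around the origin.
; PlaceRoom alternates between spawning a selector and committing it via CreateRoom, while WASD/QE move it by hex index, including up and down.
; Key 2 hands possession to the frog character with a camera blend and hides the grid.
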(event EventBeginPlay
  (CallFunction|PlaceRoom)
  (CallFunction|PlaceRoom)
  ;[0.15 0.15 0.15 0.5] Create placement grid
  (for _array_element (Utilities|Array|MakeArray -1 0 1)
    (for _array_element_2 (Utilities|Array|MakeArray -1 0 1)
      (if (Class|RoomManager|IsIndexValid (Utilities|Struct|MakeHexIndex _array_element _array_element_2))
        (bind _returnvalue (Game|SpawnActorfromClass "/Game/Rooms/BP_GridRoom.BP_GridRoom_C" (Transformation|GetActorTransform) "AlwaysSpawn" "MultiplyWithRoot" 0 0))
        (bind _returnvalue_2 (Transformation|AttachComponentToComponent _returnvalue (Variables|Default|GetGrid) "None" "KeepRelative" "KeepWorld" "KeepRelative" true))
        (if _returnvalue_2
          (Transformation|SetActorRelativeLocation _returnvalue (Class|RoomManager|GetRelativeLocationfromHex (Utilities|Struct|MakeHexIndex _array_element _array_element_2))))))
    (Rendering|SetVisibility (Variables|Default|GetGrid) false true)))

(event Input|KeyboardEvents|E
  (params (Key :type Key%20Structure))
  (:Pressed
    (CallFunction|ParseInput "Up")))

(event Input|KeyboardEvents|W
  (params (Key :type Key%20Structure))
  (:Pressed
    (CallFunction|ParseInput "North")))

(event Input|KeyboardEvents|A
  (params (Key :type Key%20Structure))
  (:Pressed
    (CallFunction|ParseInput "West")))

(event Input|KeyboardEvents|Q
  (params (Key :type Key%20Structure))
  (:Pressed
    (CallFunction|ParseInput "Down")))

(event Input|KeyboardEvents|S
  (params (Key :type Key%20Structure))
  (:Pressed
    (CallFunction|ParseInput "South")))

(event Input|KeyboardEvents|D
  (params (Key :type Key%20Structure))
  (:Pressed
    (CallFunction|ParseInput "East")))

(event Input|KeyboardEvents|SpaceBar
  (params (Key :type Key%20Structure))
  (:Pressed
    (CallFunction|PlaceRoom)))

(event Input|KeyboardEvents|2
  (params (Key :type Key%20Structure))
  (bind _returnvalue (Game|GetPlayerController 0))
  (:Pressed
    (bind _outactors (Actor|GetAllActorsOfClass "/Game/Blueprints/BP_FrogCharacter.BP_FrogCharacter_C"))
    (Pawn|Possess _returnvalue (Utilities|Array|Get(acopy) _outactors))
    (Game|Player|SetViewTargetwithBlend _returnvalue (Utilities|Array|Get(acopy) _outactors) 2.0 "VTBlend_Cubic" 0.5 true)
    (Rendering|SetVisibility (Variables|Default|GetGrid) false true)))

(fn ConstructionScript)

(fn PlaceRoom
  ;[0.15 0.15 0.15 0.5] Place new room
  (Utilities|IsValid (Variables|Default|GetSelectorActor)
    (:Is%20Valid
      (bind _returnvalue (Class|RoomManager|CreateRoom (Variables|Default|GetCurrentIndex) "/Game/Rooms/RoomDefinitions/DA_RoomDefinition.DA_RoomDefinition" (Variables|Default|GetSelectorActor)))
      (if _returnvalue
        (bind _asbp_room_actor (Utilities|Casting|CastToBP_RoomActor (Variables|Default|GetSelectorActor)))
        (Default|OnPlaceRoom _asbp_room_actor)
        (Variables|Default|SetSelectorActor 0)))
    (:Is%20Not%20Valid
      ;[0.15 0.15 0.15 0.5] Begin placing room
      (bind _returnvalue_2 (Game|SpawnActorfromClass "/Game/Rooms/BP_RoomActor.BP_RoomActor_C" (Transformation|GetActorTransform) "Undefined" "MultiplyWithRoot" 0 0))
      (bind _output_get (Variables|Default|SetSelectorActor _returnvalue_2))
      (Transformation|AttachComponentToComponent _output_get (Variables|Default|GetDefaultSceneRoot) "None" "KeepRelative" "KeepWorld" "KeepRelative" false)
      (Transformation|SetActorRelativeLocation (Variables|Default|GetSelectorActor)))))

(fn ParseInput
  (params (Input :type ERoomInputDirection%20Enum :default "North"))
  (Utilities|IsValid (Variables|Default|GetSelectorActor)
    (:Is%20Valid
      (Class|RoomManager|MoveSelector Input)
      ;[0.15 0.15 0.15 0.5] Receive Input
      (Utilities|IsValid (Variables|Default|GetSelectorActor)
        (:Is%20Valid
          (Transformation|SetRelativeLocation (Variables|/Script/Engine.Actor|GetRootComponent (Variables|Default|GetSelectorActor)) (Class|RoomManager|GetRelativeLocationfromHex (Variables|Default|GetCurrentIndex)) false false))))))