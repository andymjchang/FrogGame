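; Room actor composed of child-actor wall and floor dynamic meshes, shown with a placement material until it is placed.
; OnPlaceRoom swaps the placing material for stone wall and floor materials on both meshes.
; SetWallArray, which accepts only six-element arrays, and SetDoorArray pass layout data to BP_WallMesh, which regenerates its walls or doors.
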(event Custom|OnPlaceRoom
  (CallFunction|SetMaterial "/Game/Assets/Materials/MI_StoneWall.MI_StoneWall" "/Game/Assets/Materials/MI_StoneFloor.MI_StoneFloor"))

(event EventBeginPlay
  (CallFunction|SetMaterial "/Game/Rooms/Materials/MI_PlacingRoom.MI_PlacingRoom" "/Game/Rooms/Materials/MI_PlacingRoom.MI_PlacingRoom"))

(event EventSetDoorArray
  (params (InputArray :type Array%20of%20EDoorTypes%20Enums :default "Door"))
  ;[0.15 0.15 0.15 0.5] Set door array
  (bind _asbp_wall_mesh (Utilities|Casting|CastToBP_WallMesh (Variables|/Script/Engine.ChildActorComponent|GetChildActor (Variables|Default|GetBP_WallMesh))))
  (Variables|/Game/Rooms/BP_WallMesh.BP_WallMesh_C|SetDoorArray _asbp_wall_mesh InputArray)
  (Default|GenerateDoors _asbp_wall_mesh))

(event EventSetWallArray
  (params (InputArray :type Array%20of%20Booleans))
  ;[0.15 0.15 0.15 0.5] Set wall array on wall mesh
  (if (== (Utilities|Array|Length InputArray) 6)
    (bind _asbp_wall_mesh (Utilities|Casting|CastToBP_WallMesh (Variables|/Script/Engine.ChildActorComponent|GetChildActor (Variables|Default|GetBP_WallMesh))))
    (Variables|/Game/Rooms/BP_WallMesh.BP_WallMesh_C|SetWallArray _asbp_wall_mesh InputArray)
    (Default|GenerateWalls _asbp_wall_mesh)))

(fn ConstructionScript)

(fn SetMaterial
  (params (WallMaterial :type Material%20Instance%20Object%20Reference) (FloorMaterial :type Material%20Instance%20Object%20Reference))
  ;[0.15 0.15 0.15 0.5] Wall
  (bind _asdynamic_mesh_actor (Utilities|Casting|CastToDynamicMeshActor (Variables|/Script/Engine.ChildActorComponent|GetChildActor (Variables|Default|GetBP_WallMesh))))
  (Rendering|Material|SetMaterial (Variables|/Script/GeometryFramework.DynamicMeshActor|GetDynamicMeshComponent _asdynamic_mesh_actor) 0 WallMaterial)
  ;[0.15 0.15 0.15 0.5] Floor
  (bind _asdynamic_mesh_actor_2 (Utilities|Casting|CastToDynamicMeshActor (Variables|/Script/Engine.ChildActorComponent|GetChildActor (Variables|Default|GetBP_FloorMesh))))
  (Rendering|Material|SetMaterial (Variables|/Script/GeometryFramework.DynamicMeshActor|GetDynamicMeshComponent _asdynamic_mesh_actor_2) 0 FloorMaterial))