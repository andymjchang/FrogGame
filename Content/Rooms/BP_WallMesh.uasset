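; Hexagonal room wall actor that builds its mesh at runtime with Geometry Script booleans.
; GenerateMesh, run on BeginPlay, subtracts an inner extruded hexagon from an outer one.
; GenerateDoors cuts box openings per DoorArray entry, adds child actors for blocked doors, then generates convex-hull collision.
; GenerateWalls, like GenerateDoors not called here, places window meshes on flagged sides and cuts the others down to short-wall height.
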(event Custom|GenerateWalls
  ;[0.15 0.15 0.15 0.5] Generate Walls
  (CallFunction|DeleteAllChildren (Variables|Default|GetInstancedWindows))
  (for (_array_element _array_index) (Variables|Default|GetWallArray)
    (if _array_element
      (bind _rotation (CallFunction|GetArrayRotation _array_index))
      (bind _returnvalue (AddComponent|AddStaticMeshComponent true (Math|Transform|MakeTransform (Math|Vector|RotateVector (Math|Vector|MakeVector (- (Variables|Default|GetSmallR) (Variables|Default|GetWallWidth)) 0.0 6e+02) _rotation) _rotation "1.400000,1.400000,1.400000")))
      (Components|StaticMesh|SetStaticMesh _returnvalue (Variables|Default|GetWindowMesh))
      (Transformation|AttachComponentToComponent _returnvalue (Variables|Default|GetInstancedWindows) "None" "KeepRelative" "KeepRelative" "KeepWorld" false)
      (else
        (bind _returnvalue_2 (DynamicMeshActor|AllocateComputeMesh))
        (bind _returnvalue_3 (GeometryScript|Primitives|AppendDisc :TargetMesh _returnvalue_2 :Transform (Math|Transform|MakeTransform (Math|Vector|MakeVector (- (Variables|Default|GetSmallR) (/ (Variables|Default|GetWallLength) 2.0)) 0.0 (Variables|Default|GetShortWallHeight)) "0.000000,180.000000,0.000000") :Radius (Variables|Default|GetWallLength) :AngleSteps 3 :Debug 0))
        (bind _returnvalue_4 (Class|GeometryScriptLibraryMeshModelingFunctions|ApplyMeshExtrudeCompatibility5p0 _returnvalue_3 (Utilities|Struct|MakeGeometryScriptMeshExtrudeOptions 1.0 (Math|Vector|MakeVector 0.0 0.0 (- (Variables|Default|GetWallHeight) (Variables|Default|GetShortWallHeight))) 1.0 true) 0))
        (bind _rotation_2 (CallFunction|GetArrayRotation _array_index))
        (bind _returnvalue_5 (Class|GeometryScriptLibraryMeshTransformFunctions|RotateMesh _returnvalue_4 _rotation_2 "0.000000,0.000000,0.000000" 0))
        (GeometryScript|Booleans|ApplyMeshBoolean :TargetMesh (Variables|Default|GetWallMesh) :ToolMesh _returnvalue_5 :Operation "Subtract" :Debug 0)))))

(event Custom|GenerateDoors
  (bind _centerwallradius (Variables|Default|GetCenterWallRadius))
  (Utilities|FlowControl|Sequence
    (:then_0
      (CallFunction|DeleteAllChildren (Variables|Default|GetInstancedDoors)))
    (:then_1
      ;[0.15 0.15 0.15 0.5] Door cube cutout
      (for (_array_element _array_index) (Variables|Default|GetDoorArray)
        (switch Utilities|FlowControl|Switch|SwitchonEDoorTypes (Utilities|Enum|ByteToEnumEDoorTypes _array_element)
          (:Door
            _)
          (:Blocked
            _))
        (if true
          (bind _returnvalue (DynamicMeshActor|AllocateComputeMesh))
          (bind _returnvalue_2 (Class|GeometryScriptLibraryMeshPrimitiveFunctions|AppendBox :TargetMesh _returnvalue :Transform (Math|Transform|MakeTransform (Math|Vector|MakeVector _centerwallradius 0.0 (Variables|Default|GetFloorHeight))) :DimensionX (Variables|Default|GetWallWidth) :DimensionY (Variables|Default|GetDoorWidth) :DimensionZ (Variables|Default|GetDoorHeight) :Debug 0))
          (bind _rotation (CallFunction|GetArrayRotation _array_index))
          (bind _returnvalue_3 (Class|GeometryScriptLibraryMeshTransformFunctions|RotateMesh _returnvalue_2 _rotation "0.000000,0.000000,0.000000" 0))
          (GeometryScript|Booleans|ApplyMeshBoolean :TargetMesh (Variables|Default|GetWallMesh) :ToolMesh _returnvalue_3 :Operation "Subtract" :Debug 0)
          (switch Utilities|FlowControl|Switch|SwitchonEDoorTypes (Utilities|Enum|ByteToEnumEDoorTypes _array_element)
            (:Blocked
              (bind _returnvalue_4 (AddComponent|AddChildActorComponent true (Math|Transform|MakeTransform (Math|Vector|RotateVector (Math|Vector|MakeVector _centerwallradius 0.0 1.5e+02) _rotation) _rotation)))
              (Transformation|AttachComponentToComponent _returnvalue_4 (Variables|Default|GetInstancedDoors) "None" "KeepRelative" "KeepRelative" "KeepWorld" false))))))
    (:then_2
      ;[0.15 0.15 0.15 0.5] Generate collision
      (bind _returnvalue_5 (Class|GeometryScriptLibraryCollisionFunctions|GenerateCollisionfromMesh (Variables|Default|GetWallMesh) (Utilities|Struct|MakeGeometryScriptCollisionfromMeshOptions true "ConvexHulls" true true true 1.0 true 25 16) 0))
      (Class|GeometryScriptLibraryCollisionFunctions|SetSimpleCollisionOfDynamicMeshComponent :SimpleCollision _returnvalue_5 :DynamicMeshComponent (Variables|DynamicMeshActor|GetDynamicMeshComponent) :Debug 0))))

(event Custom|GenerateMesh
  ;[0.15 0.15 0.15 0.5] Reset mesh
  (bind _returnvalue (DynamicMeshComponent|GetDynamicMesh (Variables|DynamicMeshActor|GetDynamicMeshComponent)))
  (DynamicMesh|Reset _returnvalue)
  (Class|GeometryScriptLibraryCollisionFunctions|ResetDynamicMeshCollision (Variables|DynamicMeshActor|GetDynamicMeshComponent) false 0)
  (Variables|Default|SetSmallR (Math|Float|Sqrt (- (Math|Float|Square (Variables|Default|GetRoomRadius)) (Math|Float|Square (/ (Variables|Default|GetRoomRadius) 2.0)))))
  (Variables|Default|SetWallLength (/ (Variables|Default|GetSmallR) 1.5))
  (Variables|Default|SetWallMesh _returnvalue)
  (Variables|Default|SetCenterWallRadius (- (Variables|Default|GetSmallR) (/ (Variables|Default|GetWallWidth) 2.0)))
  (Utilities|FlowControl|Sequence
    (:then_0
      ;[0.15 0.15 0.15 0.5] Create walls
      (bind _returnvalue_2 (GeometryScript|Primitives|AppendDisc :TargetMesh (Variables|Default|GetWallMesh) :Radius (Variables|Default|GetRoomRadius) :AngleSteps 6 :Debug 0))
      (Class|GeometryScriptLibraryMeshModelingFunctions|ApplyMeshExtrudeCompatibility5p0 _returnvalue_2 (Utilities|Struct|MakeGeometryScriptMeshExtrudeOptions 1.0 (Math|Vector|MakeVector 0.0 0.0 (Variables|Default|GetWallHeight)) 1.0 true) 0))
    (:then_1
      ;[0.15 0.15 0.15 0.5] Subtract inside
      (bind _returnvalue_3 (DynamicMeshActor|AllocateComputeMesh))
      (bind _returnvalue_4 (GeometryScript|Primitives|AppendDisc :TargetMesh _returnvalue_3 :Radius (- (Variables|Default|GetRoomRadius) (Variables|Default|GetWallWidth)) :AngleSteps 6 :Debug 0))
      (bind _returnvalue_5 (Class|GeometryScriptLibraryMeshModelingFunctions|ApplyMeshExtrudeCompatibility5p0 _returnvalue_4 (Utilities|Struct|MakeGeometryScriptMeshExtrudeOptions (Variables|Default|GetWallHeight) "0.000000,0.000000,1.000000" 1.0 true) 0))
      (bind _returnvalue_6 (GeometryScript|Booleans|ApplyMeshBoolean :TargetMesh (Variables|Default|GetWallMesh) :ToolMesh _returnvalue_5 :Operation "Subtract" :Debug 0))
      (Class|GeometryScriptLibraryMeshTransformFunctions|RotateMesh _returnvalue_6 (Variables|Default|GetRotationOffset) "0.000000,0.000000,0.000000" 0))))

(event EventBeginPlay
  (CallFunction|GenerateMesh))

(fn ConstructionScript)

(fn GetArrayRotation
  (params (ArrayIndex :type Integer))
  (return (Math|Rotator|MakeRotator 0.0 0.0 (Math|Conversions|ToFloat(Integer) (+ (* ArrayIndex 60) (Variables|Default|GetDoorStartingRotation))))))

(fn DeleteAllChildren
  (params (Component :type Scene%20Component%20Object%20Reference))
  (bind _arrayelement (Utilities|Array|ReverseforEachLoop (Components|GetChildrenComponents Component false))
    (:LoopBody
      (Components|DestroyComponent _arrayelement))))