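; GA_Knockback is a shared Gameplay Ability that knocks its owning character away from whoever instigated the triggering gameplay event.
; On event activation it launches the avatar Character along the direction from the instigator to a point slightly above the avatar, adding upward lift.
; The event magnitude sets the launch speed, which overrides existing velocity on all axes, and the ability ends immediately after the launch.
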(event Ability|EventActivateAbilityFromEvent
  (params (EventData :type Gameplay%20Event%20Data%20Structure%20%28by%20ref%29))
  (bind (_eventtag _instigator _target _optionalobject _optionalobject2 _contexthandle _instigatortags _targettags _eventmagnitude) (Utilities|Struct|BreakGameplayEventData EventData))
  (bind _returnvalue (Ability|GetAvatarActorfromActorInfo))
  (Utilities|IsValid _returnvalue
    (:Is%20Valid
      (bind _ascharacter (Utilities|Casting|CastToCharacter _returnvalue))
      ;[0.15 0.15 0.15 0.5] Launch character in opposite direction
      (Character|LaunchCharacter _ascharacter (* (Math|Vector|GetUnitDirection(Vector) (Transformation|GetActorLocation _instigator) (+ (Transformation|GetActorLocation _ascharacter) "0.000000,0.000000,100.000000")) _eventmagnitude) true true)
      (Ability|EndAbility))))