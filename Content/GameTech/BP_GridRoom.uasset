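; BP_GridRoom is an actor that procedurally generates a hexagonal room block at runtime.
; On BeginPlay, GenerateMesh uses Geometry Script on its DynamicMeshComponent to append a six-step disc sized by RoomRadius.
; The disc is extruded upward by FloorHeight, then rotated 30 degrees to set the hexagon's orientation.
; The construction script is empty, so the mesh is not built there.
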(event Custom|GenerateMesh
  (bind _returnvalue (DynamicMeshComponent|GetDynamicMesh (Variables|DynamicMeshActor|GetDynamicMeshComponent)))
  (Variables|Default|SetWallMesh _returnvalue)
  ;[0.15 0.15 0.15 0.5] Create walls
  (bind _returnvalue_2 (GeometryScript|Primitives|AppendDisc :TargetMesh (Variables|Default|GetWallMesh) :Radius (Variables|Default|GetRoomRadius) :AngleSteps 6 :Debug 0))
  (bind _returnvalue_3 (Class|GeometryScriptLibraryMeshModelingFunctions|ApplyMeshExtrudeCompatibility5p0 _returnvalue_2 (Utilities|Struct|MakeGeometryScriptMeshExtrudeOptions 1.0 (Math|Vector|MakeVector 0.0 0.0 (Variables|Default|GetFloorHeight)) 1.0 true) 0))
  (Class|GeometryScriptLibraryMeshTransformFunctions|RotateMesh _returnvalue_3 "0.000000,-30.000000,0.000000" "0.000000,0.000000,0.000000" 0))

(event EventBeginPlay
  (CallFunction|GenerateMesh))

(fn ConstructionScript)