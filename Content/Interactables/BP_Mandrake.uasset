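; BP_Mandrake is an AI-controlled mandrake interactable that begins fleeing when its flee hitbox is overlapped.
; On overlap it detaches from its parent, keeping its world transform, and sets the hitbox to query-only collision.
; It then starts the StateTree on its AIC_Mandrake controller and sends it a flee event.
; EndPlay stops that StateTree logic and prints debug strings.
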(event OnComponentBeginOverlap(FleeHitbox)
  (params (OverlappedComponent :type Primitive%20Component%20Object%20Reference) (OtherActor :type Actor%20Object%20Reference) (OtherComp :type Primitive%20Component%20Object%20Reference) (OtherBodyIndex :type Integer) (bFromSweep :type Boolean) (SweepResult :type Hit%20Result%20Structure%20%28by%20ref%29))
  (Transformation|DetachFromActor "KeepWorld" "KeepWorld" "KeepWorld")
  (Collision|SetCollisionEnabled (Variables|Default|GetFleeHitbox) "QueryOnly")
  (bind _asaic_mandrake (Utilities|Casting|CastToAIC_Mandrake (Pawn|GetController)))
  (AI|Logic|StartLogic (Variables|/Game/AI/AIC_Mandrake.AIC_Mandrake_C|GetStateTreeAI _asaic_mandrake))
  (Gameplay|StateTree|SendStateTreeEvent (Variables|/Game/AI/AIC_Mandrake.AIC_Mandrake_C|GetStateTreeAI _asaic_mandrake) (Utilities|Struct|MakeStateTreeEvent "(TagName=\"AI.Event.Flee\")") :!class /Script/GameplayStateTreeModule.StateTreeComponent))

(event EventEndPlay
  (params (EndPlayReason :type EEndPlayReason%20Enum :default "Destroyed"))
  (Development|PrintString "End Play")
  (bind _asaic_mandrake (Utilities|Casting|CastToAIC_Mandrake (Pawn|GetController)))
  (Development|PrintString "loagsdaf")
  (AI|Logic|StopLogic (Variables|/Game/AI/AIC_Mandrake.AIC_Mandrake_C|GetStateTreeAI _asaic_mandrake) ""))

(fn ConstructionScript)