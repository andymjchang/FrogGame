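; Player frog character Blueprint with a nametag and a few hotkeys for debugging, switching to room placement and quitting.
; BeginPlay sets the view target to the frog and fills its nametag widget with the Steam persona name of player controller 0.
; Key 2 hands possession to the first BP_RoomManager, blending the camera over and revealing its placement grid.
; Key 1 runs the ability system debug display; Escape quits the game.
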(event EventBeginPlay
  (Game|Player|SetViewTargetwithBlend (Game|GetPlayerController 0) self 0.0 "VTBlend_Linear" 0.0 true)
  (CallFunction|SetNametag))

(event Input|KeyboardEvents|2
  (params (Key :type Key%20Structure :default "None"))
  (bind _returnvalue (Game|GetPlayerController 0))
  ;[0.15 0.15 0.15 0.5] Give control to room manager
  (:Pressed
    (bind _outactors (Actor|GetAllActorsOfClass "/Game/Rooms/BP_RoomManager.BP_RoomManager_C"))
    (Utilities|IsValid (Utilities|Array|Get(acopy) _outactors)
      (:Is%20Valid
        (Pawn|Possess _returnvalue (Utilities|Array|Get(acopy) _outactors))
        (Game|Player|SetViewTargetwithBlend _returnvalue (Utilities|Array|Get(acopy) _outactors) 2.0 "VTBlend_Cubic" 1.0 true)
        (Rendering|SetVisibility (Variables|/Game/Rooms/BP_RoomManager.BP_RoomManager_C|GetPlacementGridAttachPoint (Utilities|Array|Get(acopy) _outactors)) true true)))))

(event Input|KeyboardEvents|1
  (params (Key :type Key%20Structure :default "None"))
  (:Pressed
    (Development|ExecuteConsoleCommand "showdebug abilitysystem" 0)))

(event Input|KeyboardEvents|Escape
  (params (Key :type Key%20Structure :default "None"))
  (:Pressed
    (Game|QuitGame (Game|GetPlayerController 0) "Quit" false)))

(fn ConstructionScript)

(fn SetNametag
  ;[0.15 0.15 0.15 0.5] Set player name on nametag
  (bind _returnvalue (Class|AdvancedSteamFriendsLibrary|GetSteamPersonaName (Class|AdvancedSessionsLibrary|GetUniqueNetID (Game|GetPlayerController 0))))
  (bind _asnametag_widget (Utilities|Casting|CastToNametagWidget (UserInterface|GetWidget (Variables|Default|GetNametagWidgetComponent))))
  (Class|NametagWidget|SetPlayerName _asnametag_widget _returnvalue))