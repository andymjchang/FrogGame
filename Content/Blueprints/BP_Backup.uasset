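; BP_Backup is a player character Blueprint with a hitbox attack and an unfinished or disconnected tongue grapple, and it adds the GUI widget on BeginPlay.
; Left click briefly enables and shows the hitbox.
; Holding Left Ctrl raises walk speed, lowers the sphere and keeps the hitbox active.
; The grapple logic (camera trace, flying mode, steerable pull force) has no triggering events, so it never runs.
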(event EventBeginPlay
  ;[0.15 0.15 0.15 0.5] Begin Play
  (bind _returnvalue (UserInterface|CreateWidget "/Game/GUI/WBP_GUI.WBP_GUI_C"))
  (UserInterface|Viewport|AddtoViewport _returnvalue 0)
  (Components|Activation|SetActive (Variables|Default|GetHitbox) false false))

(event EventTick
  (params (DeltaSeconds :type Float%20%28single-precision%29))
  ;[0.15 0.15 0.15 0.5] Tick
)

(event Input|MouseEvents|RightMouseButton
  (params (Key :type Key%20Structure))
  ;[0.15 0.15 0.15 0.5] Grapple Event
)

(event Input|MouseEvents|LeftMouseButton
  (params (Key :type Key%20Structure))
  (bind _hitbox (Variables|Default|GetHitbox))
  (bind _hitbox_2 (Variables|Default|GetHitbox))
  ;[0.15 0.15 0.15 0.5] Attack
  (:Pressed
    (Collision|SetCollisionEnabled _hitbox "QueryOnly")
    (Development|SetHiddeninGame _hitbox false false)
    (Utilities|FlowControl|Delay 0.2)
    (Collision|SetCollisionEnabled _hitbox_2 "NoCollision")
    (Development|SetHiddeninGame _hitbox_2 true false)))

(event Input|KeyboardEvents|LeftCtrl
  (params (Key :type Key%20Structure))
  (bind _hitbox (Variables|Default|GetHitbox))
  (bind _hitbox_2 (Variables|Default|GetHitbox))
  (:Pressed
    (Variables|/Script/Engine.CharacterMovementComponent|SetMaxWalkSpeed (Variables|Character|GetCharacterMovement) 1e+03)
    (Transformation|AddLocalOffset (Variables|Default|GetSphere) "0.000000,0.000000,-40.000000" false false)
    (Collision|SetCollisionEnabled _hitbox_2 "QueryOnly")
    (Development|SetHiddeninGame _hitbox_2 false false))
  (:Released
    (Variables|/Script/Engine.CharacterMovementComponent|SetMaxWalkSpeed (Variables|Character|GetCharacterMovement) 5e+02)
    (Transformation|AddLocalOffset (Variables|Default|GetSphere) "0.000000,0.000000,40.000000" false false)
    (Collision|SetCollisionEnabled _hitbox "NoCollision")
    (Development|SetHiddeninGame _hitbox true false)))

(fn ConstructionScript)