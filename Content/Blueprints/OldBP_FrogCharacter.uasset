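; Player frog character Blueprint that carries, drops and picks up ingredient items and casts a channeled fireball spell.
; Hidden cube components mark the held item; E spawns that ingredient in front, or briefly enables a pickup hitbox when empty-handed.
; A spell key spawns magic circle and fireball effects with a montage and timed hover.
; BeginPlay puts the Steam name on the healthbar widget; other keys show a book, inventory and ability debug, or quit.
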(event EventBeginPlay
  ;[0.15 0.15 0.15 0.5] Set player name on nametag
  (bind _returnvalue (Class|AdvancedSteamFriendsLibrary|GetSteamPersonaName (Class|AdvancedSessionsLibrary|GetUniqueNetID (Game|GetPlayerController 0))))
  (bind _aswbp_ally_healthbar (Utilities|Casting|CastToWBP_AllyHealthbar (UserInterface|GetWidget (Variables|Default|GetHealthBarWidgetComponent))))
  (Default|SetPlayerName _aswbp_ally_healthbar _returnvalue)
  (GameplayAbilities|GiveAbility (Variables|Default|GetAbilitySystemComponent) 0 0 -1)
  (Rendering|SetVisibility (Variables|Default|GetCube) false false)
  (Rendering|SetVisibility (Variables|Default|GetBlueCube) false false)
  (Rendering|SetVisibility (Variables|Default|GetCompleteCube) false false)
  (Rendering|SetVisibility (Variables|Default|GetBook) false false)
  (Collision|SetCollisionEnabled (Variables|Default|GetItemPickupHitbox) "NoCollision"))

(event Input|KeyboardEvents|Escape
  (params (Key :type Key%20Structure :default "None"))
  ;[0.15 0.15 0.15 0.5] Quit game
  (:Pressed
    (Game|QuitGame 0 "Quit" false)))

(event Input|KeyboardEvents|4
  (params (Key :type Key%20Structure :default "None"))
  ;[0.15 0.15 0.15 0.5] Print inventory
  (:Pressed
    (Development|PrintString "Inventory:")
    (for _array_element (Variables|Default|GetItems (Variables|Default|GetInventoryComponent))
      (Development|PrintString (Utilities|GetDisplayName _array_element)))))

(event Input|KeyboardEvents|1
  (params (Key :type Key%20Structure :default "None"))
  ;[0.15 0.15 0.15 0.5] Show ability system debug
  (:Pressed
    (Development|ExecuteConsoleCommand "ShowDebug AbilitySystem" (Game|GetPlayerController 0))))

(event Input|KeyboardEvents|3
  (params (Key :type Key%20Structure :default "None"))
  (:Pressed
    (bind _returnvalue (CallFunction|GetFloorLocation))
    (Game|SpawnActorfromClass "/Game/FabContent/FXVarietyPack/Blueprints/BP_ky_magicCircle1.BP_ky_magicCircle1_C" (Math|Conversions|ToTransform(Vector) _returnvalue) "AlwaysSpawn" "MultiplyWithRoot" 0 0)
    (Game|SpawnActorfromClass "/Game/FabContent/FXVarietyPack/Blueprints/BP_ky_fireBall.BP_ky_fireBall_C" (Math|Conversions|ToTransform(Vector) (+ (Transformation|GetActorLocation) "0.000000,0.000000,100.000000")) "AlwaysSpawn" "MultiplyWithRoot" 0 0)
    (Animation|Montage|PlayMontage (Variables|Character|GetMesh) "/Game/Assets/AM_FrogChannel.AM_FrogChannel"
      (:then
        (Pawn|Components|CharacterMovement|SetMovementMode (Variables|Character|GetCharacterMovement) "MOVE_Flying" 0)
        (Physics|AddImpulse (Variables|Character|GetCharacterMovement) "0.000000,0.000000,10000.000000" false)
        (Utilities|FlowControl|Delay 1.5)
        (Physics|AddImpulse (Variables|Character|GetCharacterMovement) "0.000000,0.000000,-10000.000000" false)
        (Pawn|Components|CharacterMovement|SetMovementMode (Variables|Character|GetCharacterMovement) "MOVE_Falling" 0)))))

(event Input|KeyboardEvents|4
  (params (Key :type Key%20Structure :default "None"))
  (:Pressed
    (Rendering|SetVisibility (Variables|Default|GetBook) true false)))

(event Input|KeyboardEvents|E
  (params (Key :type Key%20Structure :default "None"))
  (bind _returnvalue (Transformation|GetActorLocation))
  (bind _returnvalue_2 (Transformation|GetActorForwardVector))
  (bind _cube (Variables|Default|GetCube))
  (bind _completecube (Variables|Default|GetCompleteCube))
  (bind _returnvalue_3 (* _returnvalue_2 1e+02))
  (bind _returnvalue_4 (+ _returnvalue _returnvalue_3))
  (bind _returnvalue_5 (Math|Conversions|ToTransform(Vector) _returnvalue_4))
  (:Pressed
    (Variables|Default|SetIsPuttingDown false)
    (if (Variables|/Script/Engine.SceneComponent|GetbVisible (Variables|Default|GetBlueCube))
      (Variables|Default|SetIsPuttingDown true)
      (Rendering|SetVisibility (Variables|Default|GetBlueCube) false false)
      (Game|SpawnActorfromClass "/Game/Blueprints/Prototype/BP_Ingredient2.BP_Ingredient2_C" _returnvalue_5 "Undefined" "MultiplyWithRoot" 0 0))
    (if (Variables|/Script/Engine.SceneComponent|GetbVisible _cube)
      (Variables|Default|SetIsPuttingDown true)
      (Rendering|SetVisibility _cube false false)
      (Game|SpawnActorfromClass "/Game/Blueprints/Prototype/BP_Ingredient.BP_Ingredient_C" _returnvalue_5 "Undefined" "MultiplyWithRoot" 0 0))
    (if (Variables|/Script/Engine.SceneComponent|GetbVisible _completecube)
      (Variables|Default|SetIsPuttingDown true)
      (Rendering|SetVisibility _completecube false false)
      (Game|SpawnActorfromClass "/Game/Blueprints/Prototype/BP_CompleteIngredient.BP_CompleteIngredient_C" _returnvalue_5 "Undefined" "MultiplyWithRoot" 0 0))
    (if (not (Variables|Default|GetIsPuttingDown))
      (Collision|SetCollisionEnabled (Variables|Default|GetItemPickupHitbox) "QueryOnly")))
  (:Released
    (Collision|SetCollisionEnabled (Variables|Default|GetItemPickupHitbox) "NoCollision")))

(fn ConstructionScript)