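; BP_PortalDown is a prototype portal actor that moves the frog character when it overlaps the portal's sphere.
; On overlap it records the frog's location and plays a timeline, teleporting the frog each update to that location plus the timeline's position offset.
; A separate BroadcastToFloors event, not called within this graph, shows BP_Room actors below the player pawn and hides the rest.
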(event OnComponentBeginOverlap(Sphere1)
  (params (OverlappedComponent :type Primitive%20Component%20Object%20Reference) (OtherActor :type Actor%20Object%20Reference) (OtherComp :type Primitive%20Component%20Object%20Reference) (OtherBodyIndex :type Integer) (bFromSweep :type Boolean) (SweepResult :type Hit%20Result%20Structure%20%28by%20ref%29))
  (bind _asbp_frog_character (Utilities|Casting|CastToBP_FrogCharacter OtherActor))
  (Variables|Default|SetOriginalLocation (Transformation|GetActorLocation _asbp_frog_character))
  (bind _position (Timeline|Timeline Play)
    (:Update
      (Transformation|SetActorLocation _asbp_frog_character (+ (Variables|Default|GetOriginalLocation) _position) false true))))

(event Custom|BroadcastToFloors
  (bind _outactors (Actor|GetAllActorsOfClass "/Game/Blueprints/Prototype/BP_Room.BP_Room_C"))
  (for _array_element _outactors
    (if (< (.Z (Math|Vector|BreakVector (Transformation|GetWorldLocation (Variables|/Game/Blueprints/Prototype/BP_Room.BP_Room_C|GetDefaultSceneRoot _array_element)))) (.Z (Math|Vector|BreakVector (Transformation|GetActorLocation (Game|Player|GetPlayerPawn 0)))))
      (Rendering|SetVisibility (Variables|/Game/Blueprints/Prototype/BP_Room.BP_Room_C|GetDefaultSceneRoot _array_element) true true)
      (else
        (Rendering|SetVisibility (Variables|/Game/Blueprints/Prototype/BP_Room.BP_Room_C|GetDefaultSceneRoot _array_element) false true)))))

(event EventBeginPlay)

(event Collision|EventActorBeginOverlap
  (params (OtherActor :type Actor%20Object%20Reference)))

(event EventTick
  (params (DeltaSeconds :type Float%20%28single-precision%29)))

(fn ConstructionScript)