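; BP_Cauldron is a prototype cauldron that combines two ingredient types into a completed ingredient.
; Sphere overlaps destroy a BP_Ingredient or BP_Ingredient2 and reveal Green or Blue respectively, using component visibility as the record of what it holds.
; When both are visible, it spawns BP_CompleteIngredient at its own location and hides both to reset.
; An unconnected branch that toggles cube visibility never runs.
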(event OnComponentBeginOverlap(Sphere)
  (params (OverlappedComponent :type Primitive%20Component%20Object%20Reference) (OtherActor :type Actor%20Object%20Reference) (OtherComp :type Primitive%20Component%20Object%20Reference) (OtherBodyIndex :type Integer) (bFromSweep :type Boolean) (SweepResult :type Hit%20Result%20Structure%20%28by%20ref%29))
  (bind _green (Variables|Default|GetGreen))
  (bind _blue (Variables|Default|GetBlue))
  (bind _asbp_ingredient (Utilities|Casting|CastToBP_Ingredient OtherActor)
    (:then
      (Rendering|SetVisibility _green true false)
      (Actor|DestroyActor _asbp_ingredient))
    (:CastFailed
      (bind _asbp_ingredient_2 (Utilities|Casting|CastToBP_Ingredient2 OtherActor))
      (Rendering|SetVisibility _blue true false)
      (Actor|DestroyActor _asbp_ingredient_2)))
  (if (and (Variables|/Script/Engine.SceneComponent|GetbVisible _green) (Variables|/Script/Engine.SceneComponent|GetbVisible _blue))
    (Game|SpawnActorfromClass "/Game/Blueprints/Prototype/BP_CompleteIngredient.BP_CompleteIngredient_C" (Math|Conversions|ToTransform(Vector) (Transformation|GetActorLocation)) "Undefined" "MultiplyWithRoot" 0 0)
    (Rendering|SetVisibility (Variables|Default|GetGreen) false false)
    (Rendering|SetVisibility (Variables|Default|GetBlue) false false)))

(event EventBeginPlay
  (Rendering|SetVisibility (Variables|Default|GetBlue) false false)
  (Rendering|SetVisibility (Variables|Default|GetGreen) false false))

(fn ConstructionScript)