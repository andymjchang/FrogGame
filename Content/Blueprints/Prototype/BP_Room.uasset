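; Prototype room actor that lets the frog character grow the level by spending a carried book at one of six trigger components.
; On overlap, if the BP_FrogCharacter's Book is visible, it hides the book, spawns a green, blue or further BP_Room at the matching scene point, then disables that trigger's collision.
; Tick shows the room only while its root is below the player pawn, and ToggleVisible switches two meshes' visibility.
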(event OnComponentBeginOverlap(1)
  (params (OverlappedComponent :type Primitive%20Component%20Object%20Reference) (OtherActor :type Actor%20Object%20Reference) (OtherComp :type Primitive%20Component%20Object%20Reference) (OtherBodyIndex :type Integer) (bFromSweep :type Boolean) (SweepResult :type Hit%20Result%20Structure%20%28by%20ref%29))
  (bind _asbp_frog_character (Utilities|Casting|CastToBP_FrogCharacter OtherActor))
  (if (Variables|/Script/Engine.SceneComponent|GetbVisible (Variables|/Game/Blueprints/BP_FrogCharacter.BP_FrogCharacter_C|GetBook _asbp_frog_character))
    (Rendering|SetVisibility (Variables|/Game/Blueprints/BP_FrogCharacter.BP_FrogCharacter_C|GetBook _asbp_frog_character) false false)
    (Game|SpawnActorfromClass "/Game/Blueprints/Prototype/BP_GreenRoom.BP_GreenRoom_C" (Math|Conversions|ToTransform(Vector) (Transformation|GetWorldLocation (Variables|Default|GetScene1))) "Undefined" "MultiplyWithRoot" 0 0)
    (Collision|SetCollisionEnabled (Variables|Default|Get1) "NoCollision")))

(event OnComponentBeginOverlap(2)
  (params (OverlappedComponent :type Primitive%20Component%20Object%20Reference) (OtherActor :type Actor%20Object%20Reference) (OtherComp :type Primitive%20Component%20Object%20Reference) (OtherBodyIndex :type Integer) (bFromSweep :type Boolean) (SweepResult :type Hit%20Result%20Structure%20%28by%20ref%29))
  (bind _asbp_frog_character (Utilities|Casting|CastToBP_FrogCharacter OtherActor))
  (if (Variables|/Script/Engine.SceneComponent|GetbVisible (Variables|/Game/Blueprints/BP_FrogCharacter.BP_FrogCharacter_C|GetBook _asbp_frog_character))
    (Rendering|SetVisibility (Variables|/Game/Blueprints/BP_FrogCharacter.BP_FrogCharacter_C|GetBook _asbp_frog_character) false false)
    (Game|SpawnActorfromClass "/Game/Blueprints/Prototype/BP_BlueRoom.BP_BlueRoom_C" (Math|Conversions|ToTransform(Vector) (Transformation|GetWorldLocation (Variables|Default|GetScene2))) "Undefined" "MultiplyWithRoot" 0 0)
    (Collision|SetCollisionEnabled (Variables|Default|Get2) "NoCollision")))

(event OnComponentBeginOverlap(3)
  (params (OverlappedComponent :type Primitive%20Component%20Object%20Reference) (OtherActor :type Actor%20Object%20Reference) (OtherComp :type Primitive%20Component%20Object%20Reference) (OtherBodyIndex :type Integer) (bFromSweep :type Boolean) (SweepResult :type Hit%20Result%20Structure%20%28by%20ref%29))
  (bind _asbp_frog_character (Utilities|Casting|CastToBP_FrogCharacter OtherActor))
  (if (Variables|/Script/Engine.SceneComponent|GetbVisible (Variables|/Game/Blueprints/BP_FrogCharacter.BP_FrogCharacter_C|GetBook _asbp_frog_character))
    (Rendering|SetVisibility (Variables|/Game/Blueprints/BP_FrogCharacter.BP_FrogCharacter_C|GetBook _asbp_frog_character) false false)
    (Game|SpawnActorfromClass "BP_Room_C" (Math|Conversions|ToTransform(Vector) (Transformation|GetWorldLocation (Variables|Default|GetScene3))) "Undefined" "MultiplyWithRoot" 0 0)
    (Collision|SetCollisionEnabled (Variables|Default|Get3) "NoCollision")))

(event OnComponentBeginOverlap(4)
  (params (OverlappedComponent :type Primitive%20Component%20Object%20Reference) (OtherActor :type Actor%20Object%20Reference) (OtherComp :type Primitive%20Component%20Object%20Reference) (OtherBodyIndex :type Integer) (bFromSweep :type Boolean) (SweepResult :type Hit%20Result%20Structure%20%28by%20ref%29))
  (bind _asbp_frog_character (Utilities|Casting|CastToBP_FrogCharacter OtherActor))
  (if (Variables|/Script/Engine.SceneComponent|GetbVisible (Variables|/Game/Blueprints/BP_FrogCharacter.BP_FrogCharacter_C|GetBook _asbp_frog_character))
    (Rendering|SetVisibility (Variables|/Game/Blueprints/BP_FrogCharacter.BP_FrogCharacter_C|GetBook _asbp_frog_character) false false)
    (Game|SpawnActorfromClass "BP_Room_C" (Math|Conversions|ToTransform(Vector) (Transformation|GetWorldLocation (Variables|Default|GetScene4))) "Undefined" "MultiplyWithRoot" 0 0)
    (Collision|SetCollisionEnabled (Variables|Default|Get4) "NoCollision")))

(event OnComponentBeginOverlap(5)
  (params (OverlappedComponent :type Primitive%20Component%20Object%20Reference) (OtherActor :type Actor%20Object%20Reference) (OtherComp :type Primitive%20Component%20Object%20Reference) (OtherBodyIndex :type Integer) (bFromSweep :type Boolean) (SweepResult :type Hit%20Result%20Structure%20%28by%20ref%29))
  (bind _asbp_frog_character (Utilities|Casting|CastToBP_FrogCharacter OtherActor))
  (if (Variables|/Script/Engine.SceneComponent|GetbVisible (Variables|/Game/Blueprints/BP_FrogCharacter.BP_FrogCharacter_C|GetBook _asbp_frog_character))
    (Rendering|SetVisibility (Variables|/Game/Blueprints/BP_FrogCharacter.BP_FrogCharacter_C|GetBook _asbp_frog_character) false false)
    (Game|SpawnActorfromClass "BP_Room_C" (Math|Conversions|ToTransform(Vector) (Transformation|GetWorldLocation (Variables|Default|GetScene5))) "Undefined" "MultiplyWithRoot" 0 0)
    (Collision|SetCollisionEnabled (Variables|Default|Get5) "NoCollision")))

(event OnComponentBeginOverlap(6)
  (params (OverlappedComponent :type Primitive%20Component%20Object%20Reference) (OtherActor :type Actor%20Object%20Reference) (OtherComp :type Primitive%20Component%20Object%20Reference) (OtherBodyIndex :type Integer) (bFromSweep :type Boolean) (SweepResult :type Hit%20Result%20Structure%20%28by%20ref%29))
  (bind _asbp_frog_character (Utilities|Casting|CastToBP_FrogCharacter OtherActor))
  (if (Variables|/Script/Engine.SceneComponent|GetbVisible (Variables|/Game/Blueprints/BP_FrogCharacter.BP_FrogCharacter_C|GetBook _asbp_frog_character))
    (Rendering|SetVisibility (Variables|/Game/Blueprints/BP_FrogCharacter.BP_FrogCharacter_C|GetBook _asbp_frog_character) false false)
    (Game|SpawnActorfromClass "BP_Room_C" (Math|Conversions|ToTransform(Vector) (Transformation|GetWorldLocation (Variables|Default|GetScene6))) "Undefined" "MultiplyWithRoot" 0 0)
    (Collision|SetCollisionEnabled (Variables|Default|Get6) "NoCollision")))

(event Custom|ToggleVisible
  (params (NewParam :type Boolean))
  (Rendering|SetVisibility (Variables|Default|GetCylinder) NewParam false)
  (Rendering|SetVisibility (Variables|Default|GetStaticMesh) NewParam false))

(event EventTick
  (params (DeltaSeconds :type Float%20%28single-precision%29))
  (bind _defaultsceneroot (Variables|Default|GetDefaultSceneRoot))
  (if (< (.Z (Math|Vector|BreakVector (Transformation|GetWorldLocation _defaultsceneroot))) (.Z (Math|Vector|BreakVector (Transformation|GetActorLocation (Game|Player|GetPlayerPawn 0)))))
    (Rendering|SetVisibility _defaultsceneroot true true)
    (else
      (Rendering|SetVisibility _defaultsceneroot false true))))

(fn ConstructionScript)