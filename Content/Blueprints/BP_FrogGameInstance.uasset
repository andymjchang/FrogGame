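; Game instance for the frog game that handles hosting and invite-based joining of multiplayer sessions.
; CreateSession starts destroying any existing session and, without waiting for the result, creates an advanced LAN session, then opens Test_Rooms as a listen server.
; Accepting an invite joins that session only after the old one is successfully destroyed.
; Outcomes are reported with debug prints, and the invite-received event is an empty stub.
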(event Custom|CreateSession
  (bind _returnvalue (Game|GetPlayerController 0))
  ;[0.15 0.15 0.15 0.5] Create Session
  (|DestroySession _returnvalue
    (:then
      (|AdvancedSession 0 _returnvalue 4 4 true true false true true false false false true false true
        (:OnSuccess
          (Development|PrintString "Created Session")
          (Game|OpenLevel(byName) "Test_Rooms" true "?listen"))))))

(event EventOnSessionInviteAccepted
  (params (LocalPlayerNum :type Integer) (PersonInvited :type BP%20Unique%20Net%20Id%20Structure) (SessionToJoin :type Blueprint%20Session%20Result%20Structure%20%28by%20ref%29))
  (bind _returnvalue (Game|GetPlayerController 0))
  ;[0.15 0.15 0.15 0.5] Session Invite Accepted
  (|DestroySession _returnvalue
    (:OnSuccess
      (Development|PrintString "Try to join session")
      (|JoinSession _returnvalue SessionToJoin
        (:OnSuccess
          (Development|PrintString "Joined session"))
        (:OnFailure
          (Development|PrintString "Hell2o"))))
    (:OnFailure
      (Development|PrintString "Hello"))))

(event EventOnSessionInviteReceived
  (params (LocalPlayerNum :type Integer) (PersonInviting :type BP%20Unique%20Net%20Id%20Structure) (AppId :type String) (SessionToJoin :type Blueprint%20Session%20Result%20Structure%20%28by%20ref%29)))