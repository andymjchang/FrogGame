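; BP_Frog2 is a frog pawn with an orthographic follow camera and debug-style key bindings, and it takes the player's view on BeginPlay.
; Key 1 toggles the Ability System debug display.
; Key 2 hands possession to the first BP_RoomManager in the level and blends the view to it, while a timeline eases the frog's own FollowCamera to a wider ortho width.
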(event EventBeginPlay
  (Game|Player|SetViewTargetwithBlend (Game|GetPlayerController 0) self 0.0 "VTBlend_Linear" 0.0 true))

(event Input|KeyboardEvents|2
  (params (Key :type Key%20Structure))
  (bind _returnvalue (Game|GetPlayerController 0))
  (:Pressed
    (bind _outactors (Actor|GetAllActorsOfClass "/Game/GameTech/BP_RoomManager.BP_RoomManager_C"))
    (Utilities|IsValid (Utilities|Array|Get(acopy) _outactors)
      (:Is%20Valid
        (Pawn|Possess _returnvalue (Utilities|Array|Get(acopy) _outactors))
        (Game|Player|SetViewTargetwithBlend _returnvalue (Utilities|Array|Get(acopy) _outactors) 2.0 "VTBlend_Cubic" 1.0 true)
        (bind _orthowidth (Timeline|InterpolateOrthoWidth PlayFromStart)
          (:Update
            (Class|CameraComponent|SetOrthoWidth (Variables|Default|GetFollowCamera) (Class|KismetMathLibrary|FInterpEaseinOut 1.8e+03 3e+03 _orthowidth 1.0))))))))

(event Input|KeyboardEvents|1
  (params (Key :type Key%20Structure))
  (:Pressed
    (Development|ExecuteConsoleCommand "showdebug abilitysystem" 0)))

(fn ConstructionScript)