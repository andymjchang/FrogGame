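; BP_Frog is the frog Blueprint, which carries a nametag showing a Steam player name.
; On BeginPlay it looks up the Steam persona name of player controller 0 and passes it to the WBP_AllyHealthbar in its nametag widget component.
; The name always comes from that first controller, with no check of who controls the frog.
; The 1 key toggles the Ability System debug display through a console command.
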(event EventBeginPlay
  (CallFunction|SetSteamName))

(event Input|KeyboardEvents|1
  (params (Key :type Key%20Structure :default "None"))
  (:Pressed
    (Development|ExecuteConsoleCommand "showdebug abilitysystem" 0)))

(fn ConstructionScript)

(fn SetSteamName
  ;[0.15 0.15 0.15 0.5] Set player name on nametag
  (bind _returnvalue (Class|AdvancedSteamFriendsLibrary|GetSteamPersonaName (Class|AdvancedSessionsLibrary|GetUniqueNetID (Game|GetPlayerController 0))))
  (bind _aswbp_ally_healthbar (Utilities|Casting|CastToWBP_AllyHealthbar (UserInterface|GetWidget (Variables|Default|GetNametagWidgetComponent))))
  (Default|SetPlayerName _aswbp_ally_healthbar _returnvalue))